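; BP_DialogInteract is an interactable world object that changes game progression and triggers dialog when the player uses it.
; On Interact it adds and removes configured game stages on GM_FirstPersonGamemode, then starts the named dialog unless it is None.
; It then either destroys itself or switches off its interactable flag, which the Interactable function reports.
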(event `self.Interact`
  (params (LastPossess :type "Pawn Object Reference"))
  (bind _playdialogoncollect (`self.PlayDialogOnCollect`))
  (bind _asgm_first_person_gamemode (cast `/Game/Blueprints/GM_FirstPersonGamemode` (`GameplayStatics.GetGameMode`)))
  (for _array_element (`self.DialogStagesToAdd`)
    (`/Game/Blueprints/GM_FirstPersonGamemode.Add GameStage` _asgm_first_person_gamemode _array_element))
  (for _array_element_2 (`self.DialogStagesToRemove`)
    (`/Game/Blueprints/GM_FirstPersonGamemode.Remove GameStage` _asgm_first_person_gamemode _array_element_2))
  (bind _asgm_first_person_gamemode_2 (cast `/Game/Blueprints/GM_FirstPersonGamemode` (`GameplayStatics.GetGameMode`))
    (:`then`
      (if (not (== _playdialogoncollect "None"))
        (`/Game/Blueprints/GM_FirstPersonGamemode.StartDialog` _asgm_first_person_gamemode_2 _playdialogoncollect)))
    (:`CastFailed`
      _))
  (if (`self.DestroyObjectOnCollect`)
    (`self.K2_DestroyActor`)
    (else
      (`self.SetCanInteract` false)
      (`self.SetSelected` false))))

(event `self.SetCanInteract`
  (params (newInteractable :type Boolean))
  (set `self.isInteractable` newInteractable))

(event `self.SetSelected`
  (params (Selected :type Boolean)))

(fn `Interactable`
  (returns (IsInteractable :type Boolean))
  (return (`self.isInteractable`)))

(fn `UserConstructionScript`)