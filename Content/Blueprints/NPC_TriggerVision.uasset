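; NPC_TriggerVision is a one-shot trigger box that starts an NPC interaction and directs the player's look toward that NPC.
; It starts inactive and arms when GameStageUpdate reports the stage matching ActivateAfter.
; On overlap it sends InteractMessage to NPCToTrigger, then calls LookAtThing on BP_Player with the dialog actor's head position plus NPCOffset.
; DoOnce precedes the player check, so the first overlap by any actor while active consumes the trigger.
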(event `self.ReceiveBeginPlay`
  (set `self.active` false))

(event `self.Box.OnComponentBeginOverlap`
  (params (OverlappedComponent :type "PrimitiveComponent Object Reference") (OtherActor :type "Actor Object Reference") (OtherComp :type "PrimitiveComponent Object Reference") (OtherBodyIndex :type Integer) (bFromSweep :type Boolean) (SweepResult :type "HitResult Structure (by ref)"))
  (if (`self.active`)
    (`/Engine/EditorBlueprintResources/StandardMacros.DoOnce` false
      (:`Completed`
        (bind _aspawn (cast `Pawn` OtherActor))
        (if (== (`GameplayStatics.GetObjectClass` OtherActor) "/Game/Blueprints/BP_Player.BP_Player_C")
          (message `/Game/Blueprints/Interfaces/BPI_Interactable.Interact` (`self.NPC_ToTrigger`) _aspawn)
          (bind _asbp_player (cast `/Game/Blueprints/BP_Player` OtherActor))
          (bind _asbp_dialog_actor (cast `/Game/Blueprints/BP_DialogActor` (`self.NPC_ToTrigger`)))
          (bind _headlocation (`/Game/Blueprints/BP_DialogActor.GetHeadPosition` _asbp_dialog_actor))
          (`/Game/Blueprints/BP_Player.LookAtThing` _asbp_player (+ _headlocation (`self.NPC_Offset`))))))))

(event `/Game/Blueprints/Interfaces/BPI_GameStageListener.GameStageUpdate`
  (params (StageUpdated :type "/Game/Blueprints/DialogSystem/GameStages Enum" :default "NewEnumerator3"))
  (if (`|EnumEquality` StageUpdated (`self.ActivateAfter`))
    (set `self.active` true)))

(fn `UserConstructionScript`)