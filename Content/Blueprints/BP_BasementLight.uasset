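; Light actor that reacts to game stage updates, with a BasementLight flag selecting its behaviour.
; Basement lights start at zero intensity, then on a stage update flicker via a timed loop macro of random length, rising in brightness until they settle on with a randomised click.
; Other lights black out on the disable stage and return dim red after a random delay, or otherwise switch to bright white.
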(event `self.ReceiveBeginPlay`
  (if (`self.BasementLight`)
    (`LightComponent.SetIntensity` (`self.e`) 0.0)))

(event `/Game/Blueprints/Interfaces/BPI_GameStageListener.GameStageUpdate`
  (params (StageUpdated :type "/Game/Blueprints/DialogSystem/GameStages Enum" :default "NewEnumerator3"))
  (bind _returnvalue (`KismetMathLibrary.RandomFloat`))
  (bind _e (`self.e`))
  (bind _e_2 (`self.e`))
  (bind _e_3 (`self.e`))
  (if (`self.BasementLight`)
    (`KismetSystemLibrary.Delay` 2.0)
    (if (`|EnumEquality` StageUpdated (`self.Stage Updated`))
      (`self.LoopWithWaitTime` 0 (`KismetMathLibrary.RandomIntegerInRange` 15 40) (/ (`KismetMathLibrary.RandomFloat`) 2.0)
        (:`Exec`
          (`SceneComponent.ToggleVisibility` _e false)
          (`LightComponent.SetIntensity` _e (+ (`LightComponentBase.Intensity` _e) 0.02)))
        (:`Completed`
          (`SceneComponent.SetVisibility` _e true false)
          (`LightComponent.SetIntensity` _e 1.0)
          (`GameplayStatics.PlaySoundAtLocation` "/Game/Sounds/SFX/Click.Click" (`SceneComponent.K2_GetComponentLocation` (`self.e`)) (struct) _returnvalue (+ _returnvalue 0.5) 0.0 null null null null))))
    (elif (`|EnumEquality` StageUpdated (`self.StageDisable`))
      (`LightComponent.SetIntensity` (`self.e`) 0.0)
      (`KismetSystemLibrary.Delay` (+ (* (`KismetMathLibrary.RandomFloat`) 3.0) 2.0))
      (`LightComponent.SetIntensity` _e_2 0.5)
      (`LightComponent.SetLightColor` _e_2 (struct :`R` 1.0 :`G` 0.307292 :`B` 0.345412 :`A` 1.0) true)
      (elif (`|EnumEquality` (`self.Stage Updated`) StageUpdated)
        (`LightComponent.SetIntensity` _e_3 4.0)
        (`LightComponent.SetLightColor` _e_3 (struct :`R` 1.0 :`G` 1.0 :`B` 1.0 :`A` 1.0) true)))))

(fn `UserConstructionScript`)