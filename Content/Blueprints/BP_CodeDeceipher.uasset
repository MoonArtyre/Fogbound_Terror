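; Code-entry puzzle pawn that the player controller possesses at a specific game stage, swapping player input mapping for keypad mapping.
; Single-character key presses build a displayed code, auto-checked at full length; the single-character filter leaves Confirm and Backspace cases unreachable.
; A wrong code shows red, then resets.
; A correct code plays a sequence, enables the unlock actor, repossesses the player, removes keypad mapping and adds the next game stage.
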(event `self.ReceiveBeginPlay`)

(event `/Game/Blueprints/Interfaces/BPI_Interactable.SetSelected`
  (params (Selected :type Boolean)))

(event `/Game/Blueprints/Interfaces/BPI_GameStageListener.GameStageUpdate`
  (params (StageUpdated :type "/Game/Blueprints/DialogSystem/GameStages Enum" :default "NewEnumerator3"))
  (if (`|EnumEquality` StageUpdated "NewEnumerator18")
    (set `self.Last Possess` (`GameplayStatics.GetPlayerPawn` 0))
    (`Controller.Possess` (`GameplayStatics.GetPlayerController` 0) self)
    (message `/Game/Blueprints/Interfaces/BPI_Interactable.SetSelected` self false)
    (`self.AddMappingFunction`)))

(event `CheckCode`
  (bind _unlockactor (`self.UnlockActor`))
  (bind _sequenceactor (`self.SequenceActor`))
  ;[1 1 1] Input Code
  (if (`KismetStringLibrary.EqualEqual_StrStr` (`self.CurrrentCode`) (`self.WantedCode`)) :!label _label
    (`TextRenderComponent.K2_SetText` (`self.Input Code`) "Correct!")
    (`TextRenderComponent.SetTextRenderColor` (`self.Input Code`) (make `Color` 0 255 0 255))
    (set `self.CanInteract` false)
    (`|ExecutionSequence`
      (:`then_0`
        (`/Engine/EditorBlueprintResources/StandardMacros.IsValid` _sequenceactor
          (:`Is Valid`
            (`MovieSceneSequencePlayer.Play` (`LevelSequenceActor.SequencePlayer` _sequenceactor)))
          (:`Is Not Valid`
            (`KismetSystemLibrary.PrintString` "No Sequence Actor!"))))
      (:`then_1`
        (`/Engine/EditorBlueprintResources/StandardMacros.IsValid` _unlockactor
          (:`Is Valid`
            (message `/Game/Blueprints/Interfaces/BPI_Interactable.SetCanInteract` _unlockactor true))))
      (:`then_2`
        (bind _asbp_player (cast `/Game/Blueprints/BP_Player` (`self.Last Possess`)))
        (`/Game/Blueprints/BP_Player.Possess Player` _asbp_player)
        (`EnhancedInputSubsystemInterface.RemoveMappingContext` (pcsubsystem `EnhancedInputLocalPlayerSubsystem` (`GameplayStatics.GetPlayerController` 0)) "/Game/Inputs/Keypad_Inputs/IMC_Keypad.IMC_Keypad" (struct))
        (bind _asgm_first_person_gamemode (cast `/Game/Blueprints/GM_FirstPersonGamemode` (`GameplayStatics.GetGameMode`)))
        (`/Game/Blueprints/GM_FirstPersonGamemode.Add GameStage` _asgm_first_person_gamemode "NewEnumerator19")))
    (else
      (`TextRenderComponent.K2_SetText` (`self.Input Code`) "WRONG")
      (`TextRenderComponent.SetTextRenderColor` (`self.Input Code`) (make `Color` 0 0 255 255))
      (set `self.CanInteract` false)
      (`KismetSystemLibrary.Delay` 1.0)
      (bind _output_get (set `self.CurrrentCode` ""))
      (`TextRenderComponent.K2_SetText` (`self.Input Code`) (`KismetTextLibrary.Conv_StringToText` _output_get))
      (`TextRenderComponent.SetTextRenderColor` (`self.Input Code`) (make `Color` 255 255 255 255))
      (set `self.CanInteract` true))))

(event `Key|AnyKey`
  (params (Key :type "Key Structure"))
  (bind _returnvalue (`KismetTextLibrary.Conv_TextToString` (`KismetInputLibrary.Key_GetDisplayName` Key false)))
  ;[1 1 1] Input Code
  (:`Pressed`
    (if (`self.CanInteract`)
      (if (not (> (`KismetStringLibrary.Len` _returnvalue) 1))
        (switch `string` _returnvalue
          (:`Default`
            (if (< (`KismetStringLibrary.Len` (`self.CurrrentCode`)) (`KismetStringLibrary.Len` (`self.WantedCode`)))
              (bind _output_get (set `self.CurrrentCode` (`KismetStringLibrary.Concat_StrStr` (`self.CurrrentCode`) _returnvalue)))
              (`TextRenderComponent.K2_SetText` (`self.Input Code`) (`KismetTextLibrary.Conv_StringToText` _output_get) :!label _label_2)
              (`TextRenderComponent.SetTextRenderColor` (`self.Input Code`) (make `Color` 255 255 255 255))
              (if (== (`KismetStringLibrary.Len` (`self.CurrrentCode`)) (`KismetStringLibrary.Len` (`self.WantedCode`)))
                (`KismetSystemLibrary.Delay` 0.5)
                (`self.CheckCode`))
              (else
                (`self.CheckCode`))))
          (:`Confirm`
            (goto _label))
          (:`backspace`
            (set `self.CurrrentCode` "")
            (goto _label_2)))))))

(event `EnhancedInput|/Game/Inputs/Keypad_Inputs/IA_Exit`
  (params (ActionValue :type Boolean) (ElapsedSeconds :type "Float (double-precision)") (TriggeredSeconds :type "Float (double-precision)") (InputAction :type "InputAction Object Reference" :default "/Game/Inputs/Keypad_Inputs/IA_Exit.IA_Exit")))

(fn `AddMappingFunction`
  (bind _returnvalue (pcsubsystem `EnhancedInputLocalPlayerSubsystem` (`GameplayStatics.GetPlayerController` 0)))
  (`/Engine/EditorBlueprintResources/StandardMacros.IsValid` _returnvalue
    (:`Is Valid`
      (`EnhancedInputSubsystemInterface.AddMappingContext` _returnvalue "/Game/Inputs/Keypad_Inputs/IMC_Keypad.IMC_Keypad" 0 (struct))
      (`EnhancedInputSubsystemInterface.RemoveMappingContext` _returnvalue "/Game/Inputs/IMC_Player.IMC_Player" (struct)))))

(fn `Interactable`
  (returns (IsInteractable :type Boolean))
  (return (`self.CanInteract`)))

(fn `UserConstructionScript`
  (set `self.ButtonArray` (`|MakeArray` null null null null null null null null null null null null null null :!type "/Game/Blueprints/BP_KeypadButton Object Reference")))