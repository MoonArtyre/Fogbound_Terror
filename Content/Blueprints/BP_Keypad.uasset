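; Possessable code-entry keypad puzzle that plays a sequence when the correct code is confirmed.
; Interact possesses the keypad and swaps the player's mapping context for the keypad's.
; Directional input moves selection across a button array built in the construction script, with hard-coded jumps for the uneven bottom row.
; Selected buttons append, clear or check the code with colored text feedback; success or Exit returns control to BP_Player.
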(event `self.ReceiveBeginPlay`)

(event `/Game/Blueprints/Interfaces/BPI_Interactable.SetSelected`
  (params (Selected :type Boolean))
  (bind _bp_keypadbase (`self.BP_KeypadBase`))
  (if Selected
    (`MeshComponent.SetOverlayMaterial` _bp_keypadbase "/Game/Materials/Overlay/MI_PuzzleFresnel.MI_PuzzleFresnel")
    (else
      (`MeshComponent.SetOverlayMaterial` _bp_keypadbase null))))

(event `/Game/Blueprints/Interfaces/BPI_Interactable.Interact`
  (params (LastPossess :type "Pawn Object Reference"))
  (set `self.Last Possess` LastPossess)
  (`Controller.Possess` (`GameplayStatics.GetPlayerController` 0) self)
  (message `/Game/Blueprints/Interfaces/BPI_Interactable.SetSelected` self false)
  (`self.ResetSelection`)
  (`self.AddMappingFunction`))

(event `ResetSelection`
  (set `self.currentSelection` 0)
  (`/Game/Blueprints/BP_KeypadButton.SetSelected` (`|GetArrayItem` (`self.ButtonArray`) (`self.currentSelection`)) true))

(event `SelectButton`
  (params (Position :type Integer) (On :type Boolean))
  (`/Game/Blueprints/BP_KeypadButton.SetSelected` (`|GetArrayItem` (`self.ButtonArray`) Position) On))

(event `EnhancedInput|/Game/Inputs/Keypad_Inputs/IA_Right`
  (params (ActionValue :type Boolean) (ElapsedSeconds :type "Float (double-precision)") (TriggeredSeconds :type "Float (double-precision)") (InputAction :type "InputAction Object Reference" :default "/Game/Inputs/Keypad_Inputs/IA_Right.IA_Right"))
  (bind _currentselection (`self.currentSelection`))
  ;[1 1 1] Navigation
  (:`Started`
    (`self.SelectButton` _currentselection)
    (bind _result (`/Engine/EditorBlueprintResources/StandardMacros.IncrementInt` _currentselection)
      (:`  `
        (if (not (< _result (`KismetArrayLibrary.Array_Length` (`self.ButtonArray`))))
          (set `self.currentSelection` 0))
        (`self.SelectButton` (`self.currentSelection`) true)))))

(event `EnhancedInput|/Game/Inputs/Keypad_Inputs/IA_Left`
  (params (ActionValue :type Boolean) (ElapsedSeconds :type "Float (double-precision)") (TriggeredSeconds :type "Float (double-precision)") (InputAction :type "InputAction Object Reference" :default "/Game/Inputs/Keypad_Inputs/IA_Left.IA_Left"))
  (bind _currentselection (`self.currentSelection`))
  ;[1 1 1] Navigation
  (:`Started`
    (`self.SelectButton` _currentselection)
    (bind _result (`/Engine/EditorBlueprintResources/StandardMacros.DecrementInt` _currentselection)
      (:`  `
        (if (not (>= _result 0))
          (set `self.currentSelection` (- (`KismetArrayLibrary.Array_Length` (`self.ButtonArray`)) 1)))
        (`self.SelectButton` (`self.currentSelection`) true)))))

(event `EnhancedInput|/Game/Inputs/Keypad_Inputs/IA_Down`
  (params (ActionValue :type Boolean) (ElapsedSeconds :type "Float (double-precision)") (TriggeredSeconds :type "Float (double-precision)") (InputAction :type "InputAction Object Reference" :default "/Game/Inputs/Keypad_Inputs/IA_Down.IA_Down"))
  (bind _currentselection (`self.currentSelection`))
  (bind _returnvalue (+ _currentselection 4))
  ;[1 1 1] Navigation
  (:`Started`
    (`self.SelectButton` _currentselection)
    (if (< _currentselection 9)
      (if (< _returnvalue (`KismetArrayLibrary.Array_Length` (`self.ButtonArray`)))
        (set `self.currentSelection` _returnvalue)
        (else
          (set `self.currentSelection` 0)))
      (`self.SelectButton` (`self.currentSelection`) true)
      (elif (== _currentselection 9)
        (bind _output_get (set `self.currentSelection` 12))
        (`self.SelectButton` _output_get true)
        (elif (or (== _currentselection 10) (== _currentselection 11))
          (bind _output_get_2 (set `self.currentSelection` 13))
          (`self.SelectButton` _output_get_2 true)
          (else
            (bind _output_get_3 (set `self.currentSelection` 0))
            (`self.SelectButton` _output_get_3 true)))))))

(event `EnhancedInput|/Game/Inputs/Keypad_Inputs/IA_Up`
  (params (ActionValue :type Boolean) (ElapsedSeconds :type "Float (double-precision)") (TriggeredSeconds :type "Float (double-precision)") (InputAction :type "InputAction Object Reference" :default "/Game/Inputs/Keypad_Inputs/IA_Up.IA_Up"))
  (bind _currentselection (`self.currentSelection`))
  (bind _returnvalue (- _currentselection 4))
  ;[1 1 1] Navigation
  (:`Started`
    (`self.SelectButton` _currentselection)
    (if (== _currentselection 13)
      (bind _output_get (set `self.currentSelection` 11))
      (`self.SelectButton` _output_get true)
      (else
        (if (>= _returnvalue 0)
          (set `self.currentSelection` _returnvalue)
          (else
            (set `self.currentSelection` (- (`KismetArrayLibrary.Array_Length` (`self.ButtonArray`)) 1))))
        (`self.SelectButton` (`self.currentSelection`) true)))))

(event `EnhancedInput|/Game/Inputs/Keypad_Inputs/IA_Interact`
  (params (ActionValue :type Boolean) (ElapsedSeconds :type "Float (double-precision)") (TriggeredSeconds :type "Float (double-precision)") (InputAction :type "InputAction Object Reference" :default "/Game/Inputs/Keypad_Inputs/IA_Interact.IA_Interact"))
  (bind _sequenceactor (`self.SequenceActor`))
  (bind _value (`/Game/Blueprints/BP_KeypadButton.Value` (`|GetArrayItem` (`self.ButtonArray`) (`self.currentSelection`))))
  ;[1 1 1] Input Code
  (:`Started`
    (if (`self.CanInteract`)
      (switch `string` _value
        (:`Default`
          (if (< (`KismetStringLibrary.Len` (`self.CurrrentCode`)) (`KismetStringLibrary.Len` (`self.WantedCode`)))
            (bind _output_get (set `self.CurrrentCode` (`KismetStringLibrary.Concat_StrStr` (`self.CurrrentCode`) _value)))
            (`TextRenderComponent.K2_SetText` (`self.InputField`) (`KismetTextLibrary.Conv_StringToText` _output_get) :!label _label)
            (`TextRenderComponent.SetTextRenderColor` (`self.InputField`) (make `Color` 255 255 255 255))))
        (:`Confirm`
          (if (`KismetStringLibrary.EqualEqual_StrStr` (`self.CurrrentCode`) (`self.WantedCode`))
            (`TextRenderComponent.K2_SetText` (`self.InputField`) "Correct!")
            (`TextRenderComponent.SetTextRenderColor` (`self.InputField`) (make `Color` 0 255 0 255))
            (set `self.CanInteract` false)
            (`KismetSystemLibrary.Delay` 1.0)
            (`/Engine/EditorBlueprintResources/StandardMacros.IsValid` _sequenceactor
              (:`Is Valid`
                (`MovieSceneSequencePlayer.Play` (`LevelSequenceActor.SequencePlayer` _sequenceactor))
                (bind _asbp_player (cast `/Game/Blueprints/BP_Player` (`self.Last Possess`)))
                (`/Game/Blueprints/BP_Player.Possess Player` _asbp_player)
                (`EnhancedInputSubsystemInterface.RemoveMappingContext` (pcsubsystem `EnhancedInputLocalPlayerSubsystem` (`GameplayStatics.GetPlayerController` 0)) "/Game/Inputs/Keypad_Inputs/IMC_Keypad.IMC_Keypad" (struct)))
              (:`Is Not Valid`
                (`KismetSystemLibrary.PrintString` "No Sequence Actor!")))
            (else
              (`TextRenderComponent.K2_SetText` (`self.InputField`) "Wrong!")
              (`TextRenderComponent.SetTextRenderColor` (`self.InputField`) (make `Color` 0 0 255 255))
              (set `self.CanInteract` false)
              (`KismetSystemLibrary.Delay` 1.0)
              (bind _output_get_2 (set `self.CurrrentCode` ""))
              (`TextRenderComponent.K2_SetText` (`self.InputField`) (`KismetTextLibrary.Conv_StringToText` _output_get_2))
              (`TextRenderComponent.SetTextRenderColor` (`self.InputField`) (make `Color` 255 255 255 255))
              (set `self.CanInteract` true))))
        (:`Cancel`
          (set `self.CurrrentCode` "")
          (goto _label))))))

(event `EnhancedInput|/Game/Inputs/Keypad_Inputs/IA_Exit`
  (params (ActionValue :type Boolean) (ElapsedSeconds :type "Float (double-precision)") (TriggeredSeconds :type "Float (double-precision)") (InputAction :type "InputAction Object Reference" :default "/Game/Inputs/Keypad_Inputs/IA_Exit.IA_Exit"))
  (:`Started`
    (bind _asbp_player (cast `/Game/Blueprints/BP_Player` (`self.Last Possess`)))
    (`/Game/Blueprints/BP_Player.Possess Player` _asbp_player)
    (`EnhancedInputSubsystemInterface.RemoveMappingContext` (pcsubsystem `EnhancedInputLocalPlayerSubsystem` (`GameplayStatics.GetPlayerController` 0)) "/Game/Inputs/Keypad_Inputs/IMC_Keypad.IMC_Keypad" (struct))))

(fn `AddMappingFunction`
  (bind _returnvalue (pcsubsystem `EnhancedInputLocalPlayerSubsystem` (`GameplayStatics.GetPlayerController` 0)))
  (`/Engine/EditorBlueprintResources/StandardMacros.IsValid` _returnvalue
    (:`Is Valid`
      (`EnhancedInputSubsystemInterface.AddMappingContext` _returnvalue "/Game/Inputs/Keypad_Inputs/IMC_Keypad.IMC_Keypad" 0 (struct))
      (`EnhancedInputSubsystemInterface.RemoveMappingContext` _returnvalue "/Game/Inputs/IMC_Player.IMC_Player" (struct)))))

(fn `UserConstructionScript`
  (set `self.ButtonArray` (`|MakeArray` (`self.BP_KeypadButton001`) (`self.BP_KeypadButton002`) (`self.BP_KeypadButton003`) (`self.BP_KeypadButton004`) (`self.BP_KeypadButton005`) (`self.BP_KeypadButton006`) (`self.BP_KeypadButton007`) (`self.BP_KeypadButton008`) (`self.BP_KeypadButton009`) (`self.BP_KeypadButton010`) (`self.BP_KeypadButton011`) (`self.BP_KeypadButton012`) (`self.BP_KeypadButtonCancel13`) (`self.BP_KeypadButtonConfirm14`))))