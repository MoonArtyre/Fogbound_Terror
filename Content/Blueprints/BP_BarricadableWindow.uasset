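; BP_BarricadableWindow is an interactable window that the player can barricade once during a matching game stage.
; Barricades start hidden, and selection toggles an overlay highlight material on the main window.
; Interactable requires the game mode to report its InteractCondition stage active and the window to still be interactable.
; Interacting disables further use, reveals the barricades and notifies GM_FirstPersonGamemode through BarricadedWindow.
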(event `self.ReceiveBeginPlay`
  (`SceneComponent.SetVisibility` (`self.Barricades`) false true))

(event `/Game/Blueprints/Interfaces/BPI_Interactable.SetSelected`
  (params (Selected :type Boolean))
  (bind _mainwindow (`self.MainWindow`))
  (if Selected
    (`MeshComponent.SetOverlayMaterial` _mainwindow "/Game/Materials/Overlay/InteractMinimalist.InteractMinimalist")
    (else
      (`MeshComponent.SetOverlayMaterial` _mainwindow null))))

(event `/Game/Blueprints/Interfaces/BPI_Interactable.Interact`
  (params (LastPossess :type "Pawn Object Reference"))
  (set `self.IsInteractable` false)
  (`SceneComponent.SetVisibility` (`self.Barricades`) true true)
  (bind _asgm_first_person_gamemode (cast `/Game/Blueprints/GM_FirstPersonGamemode` (`GameplayStatics.GetGameMode`)))
  (`/Game/Blueprints/GM_FirstPersonGamemode.BarricadedWindow` _asgm_first_person_gamemode))

(fn `Interactable`
  (returns (IsInteractable :type Boolean))
  (bind _asgm_first_person_gamemode (cast `/Game/Blueprints/GM_FirstPersonGamemode` (`GameplayStatics.GetGameMode`)))
  (bind _isactive (`/Game/Blueprints/GM_FirstPersonGamemode.IsGameStageActive` _asgm_first_person_gamemode (`self.InteractCondition`)))
  (return (and _isactive (`self.IsInteractable`))))

(fn `UserConstructionScript`)