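; Interactable breaker box puzzle where the player must light every lamp to advance the game stage.
; Interacting smoothly possesses the box and enables cursor and keypad input; exiting returns control to the player.
; Each clickable switch toggles a fixed trio of lamps, while FlipFlops drive its visual state through the FlipSwitch macro.
; The solved check runs from the switch-on branch, and success disables interaction, exits and plays power-up sounds.
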(event `self.ReceiveBeginPlay`
  (for _array_element (`self.Lamps`)
    (`PrimitiveComponent.SetMaterial` _array_element 0 (`self.LampOffMaterial`))
    (`self.FlipSwitches`)
    (`KismetSystemLibrary.Delay` 0.2)
    (set `self.PlaySound` true)
    (`SceneComponent.SetVisibility` (`self.ShaderMask`) false false)))

(event `/Game/Blueprints/Interfaces/BPI_Interactable.SetSelected`
  (params (Selected :type Boolean))
  (bind _cube (`self.Cube`))
  (if Selected
    (`MeshComponent.SetOverlayMaterial` _cube "/Game/Materials/Overlay/InteractMinimalist.InteractMinimalist")
    (else
      (`MeshComponent.SetOverlayMaterial` _cube null))))

(event `EnhancedInput|/Game/Inputs/Keypad_Inputs/IA_Exit`
  (params (ActionValue :type Boolean) (ElapsedSeconds :type "Float (double-precision)") (TriggeredSeconds :type "Float (double-precision)") (InputAction :type "InputAction Object Reference" :default "/Game/Inputs/Keypad_Inputs/IA_Exit.IA_Exit"))
  (bind _returnvalue (`GameplayStatics.GetPlayerController` 0))
  ;[1 1 1] Exit
  (:`Started`
    (bind _asbp_player (cast `/Game/Blueprints/BP_Player` (`self.Last Possess`) :!label _label))
    (`/Game/Blueprints/BP_Player.Possess Player` _asbp_player)
    (`EnhancedInputSubsystemInterface.RemoveMappingContext` (pcsubsystem `EnhancedInputLocalPlayerSubsystem` _returnvalue) "/Game/Inputs/Keypad_Inputs/IMC_Keypad.IMC_Keypad" (struct))
    (set `PlayerController.bShowMouseCursor` false _returnvalue)
    (bind _asgm_first_person_gamemode (cast `/Game/Blueprints/GM_FirstPersonGamemode` (`GameplayStatics.GetGameMode`)))
    (`/Game/Blueprints/GM_FirstPersonGamemode.EnterGamePlayMode` _asgm_first_person_gamemode)
    (`SceneComponent.SetVisibility` (`self.w`) false false)
    (`SceneComponent.SetVisibility` (`self.ShaderMask`) false false)))

(event `Exit`
  ;[1 1 1] Exit
  (goto _label))

(event `/Game/Blueprints/Interfaces/BPI_Interactable.Interact`
  (params (LastPossess :type "Pawn Object Reference"))
  ;[1 1 1] Interact
  (set `self.Last Possess` LastPossess)
  (`/Game/Blueprints/BP_Macros.SmoothPosses` self 0.5
    (:`OUt`
      (message `/Game/Blueprints/Interfaces/BPI_Interactable.SetSelected` self false)
      (`self.AddMappingFunction`)
      (set `PlayerController.bShowMouseCursor` true (`GameplayStatics.GetPlayerController` 0))
      (`SceneComponent.SetVisibility` (`self.w`) true false)
      (`SceneComponent.SetVisibility` (`self.ShaderMask`) true false))))

(event `ActivateLamps`
  (params (LampID :type Integer))
  (bind _lampon (`self.LampOn`))
  (bind _output (`|GetArrayItem` (`self.Lamps`) LampID))
  ;[1 1 1] Lamp Activation
  (if (`|GetArrayItem` _lampon LampID)
    (`KismetArrayLibrary.Array_Set` _lampon LampID)
    (`PrimitiveComponent.SetMaterial` _output 0 (`self.LampOffMaterial`))
    (else
      (`KismetArrayLibrary.Array_Set` _lampon LampID true)
      (`PrimitiveComponent.SetMaterial` _output 0 (`self.LampOnMaterial`)))))

(event `CheckSolved`
  ;[1 1 1] OnSolved
  (set `self.IsSolved` true)
  (for _array_element (`self.LampOn`)
    (if (not _array_element)
      (bind _output_get (set `self.IsSolved` false))))
  (if _output_get
    (set `self.IsInteractable` false)
    (bind _asgm_first_person_gamemode (cast `/Game/Blueprints/GM_FirstPersonGamemode` (`GameplayStatics.GetGameMode`)))
    (`/Game/Blueprints/GM_FirstPersonGamemode.Add GameStage` _asgm_first_person_gamemode (`self.OnSolvedAddState`))
    (`self.Exit`)
    (`GameplayStatics.PlaySound2D` "/Game/Sounds/SFX/Communicator.Communicator" 1.0 1.0 0.0 null null)
    (`GameplayStatics.PlaySound2D` "/Game/Sounds/SFX/ElectricWobble.ElectricWobble" 1.0 1.0 0.0 null null)
    (`GameplayStatics.PlaySoundAtLocation` "/Game/Sounds/SFX/LampsTurningOn.LampsTurningOn" (`self.K2_GetActorLocation`) (struct) 1.0 1.0 0.0 null null null null)))

(event `self.Switch.OnReleased`
  (params (TouchedComponent :type "PrimitiveComponent Object Reference") (ButtonReleased :type "Key Structure"))
  ;[1 1 1] SwitchClicks
  (`self.ActivateLamps` 0)
  (`self.ActivateLamps` 2)
  (`self.ActivateLamps` 3)
  (`/Engine/EditorBlueprintResources/StandardMacros.FlipFlop` :!label _label_2
    (:`A`
      (`self.FlipSwitch` (`self.Switch`) :!label _label_3
        (:`Out`
          (`self.CheckSolved` :!label _label_4)
          (if (`self.PlaySound`)
            (`GameplayStatics.PlaySound2D` "/Game/Sounds/SFX/Click.Click" 1.0 (+ (/ (`KismetMathLibrary.RandomFloat`) 2.0) 0.5) 0.0 null null)))))
    (:`B`
      (goto _label_3 :!via `SwitchOff`))))

(event `self.Switch1.OnReleased`
  (params (TouchedComponent :type "PrimitiveComponent Object Reference") (ButtonReleased :type "Key Structure"))
  ;[1 1 1] SwitchClicks
  (`self.ActivateLamps` 9)
  (`self.ActivateLamps` 5)
  (`self.ActivateLamps` 7)
  (`/Engine/EditorBlueprintResources/StandardMacros.FlipFlop` :!label _label_5
    (:`A`
      (`self.FlipSwitch` (`self.Switch1`) :!label _label_6
        (:`Out`
          (goto _label_4))))
    (:`B`
      (goto _label_6 :!via `SwitchOff`))))

(event `FlipSwitches`
  (`|ExecutionSequence`
    (:`then_0`
      (goto _label_2))
    (:`then_1`
      (goto _label_5))
    (:`then_2`
      ;[1 1 1] SwitchClicks
      (`/Engine/EditorBlueprintResources/StandardMacros.FlipFlop` :!label _label_7
        (:`A`
          (`self.FlipSwitch` (`self.Switch2`) :!label _label_8
            (:`Out`
              (goto _label_4))))
        (:`B`
          (goto _label_8 :!via `SwitchOff`))))
    (:`then_3`
      (`/Engine/EditorBlueprintResources/StandardMacros.FlipFlop` :!label _label_9
        (:`A`
          (`self.FlipSwitch` (`self.Switch3`) :!label _label_10
            (:`Out`
              (goto _label_4))))
        (:`B`
          (goto _label_10 :!via `SwitchOff`))))
    (:`then_4`
      (`/Engine/EditorBlueprintResources/StandardMacros.FlipFlop` :!label _label_11
        (:`A`
          (`self.FlipSwitch` (`self.Switch4`) :!label _label_12
            (:`Out`
              (goto _label_4))))
        (:`B`
          (goto _label_12 :!via `SwitchOff`))))
    (:`then_5`
      (`/Engine/EditorBlueprintResources/StandardMacros.FlipFlop` :!label _label_13
        (:`A`
          (`self.FlipSwitch` (`self.Switch5`) :!label _label_14
            (:`Out`
              (goto _label_4))))
        (:`B`
          (goto _label_14 :!via `SwitchOff`))))
    (:`then_6`
      (`/Engine/EditorBlueprintResources/StandardMacros.FlipFlop` :!label _label_15
        (:`A`
          (`self.FlipSwitch` (`self.Switch6`) :!label _label_16
            (:`Out`
              (goto _label_4))))
        (:`B`
          (goto _label_16 :!via `SwitchOff`))))))

(event `self.Switch2.OnReleased`
  (params (TouchedComponent :type "PrimitiveComponent Object Reference") (ButtonReleased :type "Key Structure"))
  ;[1 1 1] SwitchClicks
  (`self.ActivateLamps` 1)
  (`self.ActivateLamps` 4)
  (`self.ActivateLamps` 8)
  (goto _label_7))

(event `self.Switch3.OnReleased`
  (params (TouchedComponent :type "PrimitiveComponent Object Reference") (ButtonReleased :type "Key Structure"))
  ;[1 1 1] SwitchClicks
  (`self.ActivateLamps` 7)
  (`self.ActivateLamps` 6)
  (`self.ActivateLamps` 3)
  (goto _label_9))

(event `self.Switch4.OnReleased`
  (params (TouchedComponent :type "PrimitiveComponent Object Reference") (ButtonReleased :type "Key Structure"))
  ;[1 1 1] SwitchClicks
  (`self.ActivateLamps` 5)
  (`self.ActivateLamps` 9)
  (`self.ActivateLamps` 3)
  (goto _label_11))

(event `self.Switch5.OnReleased`
  (params (TouchedComponent :type "PrimitiveComponent Object Reference") (ButtonReleased :type "Key Structure"))
  ;[1 1 1] SwitchClicks
  (`self.ActivateLamps` 6)
  (`self.ActivateLamps` 2)
  (`self.ActivateLamps` 3)
  (goto _label_13))

(event `self.Switch6.OnReleased`
  (params (TouchedComponent :type "PrimitiveComponent Object Reference") (ButtonReleased :type "Key Structure"))
  ;[1 1 1] SwitchClicks
  (`self.ActivateLamps` 5)
  (`self.ActivateLamps` 2)
  (`self.ActivateLamps` 3)
  (goto _label_15))

(event `self.Switch.OnBeginCursorOver`
  (params (TouchedComponent :type "PrimitiveComponent Object Reference"))
  (`MeshComponent.SetOverlayMaterial` (`self.Switch`) (`self.SwitchHoverMat`)))

(event `self.Switch.OnEndCursorOver`
  (params (TouchedComponent :type "PrimitiveComponent Object Reference"))
  (`MeshComponent.SetOverlayMaterial` (`self.Switch`) null))

(event `self.Switch1.OnBeginCursorOver`
  (params (TouchedComponent :type "PrimitiveComponent Object Reference"))
  (`MeshComponent.SetOverlayMaterial` (`self.Switch1`) (`self.SwitchHoverMat`)))

(event `self.Switch1.OnEndCursorOver`
  (params (TouchedComponent :type "PrimitiveComponent Object Reference"))
  (`MeshComponent.SetOverlayMaterial` (`self.Switch1`) null))

(event `self.Switch2.OnBeginCursorOver`
  (params (TouchedComponent :type "PrimitiveComponent Object Reference"))
  (`MeshComponent.SetOverlayMaterial` (`self.Switch2`) (`self.SwitchHoverMat`)))

(event `self.Switch2.OnEndCursorOver`
  (params (TouchedComponent :type "PrimitiveComponent Object Reference"))
  (`MeshComponent.SetOverlayMaterial` (`self.Switch2`) null))

(event `self.Switch3.OnBeginCursorOver`
  (params (TouchedComponent :type "PrimitiveComponent Object Reference"))
  (`MeshComponent.SetOverlayMaterial` (`self.Switch3`) (`self.SwitchHoverMat`)))

(event `self.Switch3.OnEndCursorOver`
  (params (TouchedComponent :type "PrimitiveComponent Object Reference"))
  (`MeshComponent.SetOverlayMaterial` (`self.Switch3`) null))

(event `self.Switch4.OnBeginCursorOver`
  (params (TouchedComponent :type "PrimitiveComponent Object Reference"))
  (`MeshComponent.SetOverlayMaterial` (`self.Switch4`) (`self.SwitchHoverMat`)))

(event `self.Switch4.OnEndCursorOver`
  (params (TouchedComponent :type "PrimitiveComponent Object Reference"))
  (`MeshComponent.SetOverlayMaterial` (`self.Switch4`) null))

(event `self.Switch5.OnBeginCursorOver`
  (params (TouchedComponent :type "PrimitiveComponent Object Reference"))
  (`MeshComponent.SetOverlayMaterial` (`self.Switch5`) (`self.SwitchHoverMat`)))

(event `self.Switch5.OnEndCursorOver`
  (params (TouchedComponent :type "PrimitiveComponent Object Reference"))
  (`MeshComponent.SetOverlayMaterial` (`self.Switch5`) null))

(event `self.Switch6.OnBeginCursorOver`
  (params (TouchedComponent :type "PrimitiveComponent Object Reference"))
  (`MeshComponent.SetOverlayMaterial` (`self.Switch6`) (`self.SwitchHoverMat`)))

(event `self.Switch6.OnEndCursorOver`
  (params (TouchedComponent :type "PrimitiveComponent Object Reference"))
  (`MeshComponent.SetOverlayMaterial` (`self.Switch6`) null))

(fn `AddMappingFunction`
  (bind _returnvalue (pcsubsystem `EnhancedInputLocalPlayerSubsystem` (`GameplayStatics.GetPlayerController` 0)))
  (`/Engine/EditorBlueprintResources/StandardMacros.IsValid` _returnvalue
    (:`Is Valid`
      (`EnhancedInputSubsystemInterface.AddMappingContext` _returnvalue "/Game/Inputs/Keypad_Inputs/IMC_Keypad.IMC_Keypad" 0 (struct))
      (`EnhancedInputSubsystemInterface.RemoveMappingContext` _returnvalue "/Game/Inputs/IMC_Player.IMC_Player" (struct)))))

(fn `Interactable`
  (returns (IsInteractable :type Boolean))
  (return (`self.IsInteractable`)))

(fn `UserConstructionScript`
  (bind _lamps (`self.Lamps`))
  (`KismetArrayLibrary.Array_AddUnique` _lamps (`self.Lamp10`))
  (`KismetArrayLibrary.Array_AddUnique` _lamps (`self.Lamp9`))
  (`KismetArrayLibrary.Array_AddUnique` _lamps (`self.Lamp8`))
  (`KismetArrayLibrary.Array_AddUnique` _lamps (`self.Lamp7`))
  (`KismetArrayLibrary.Array_AddUnique` _lamps (`self.Lamp6`))
  (`KismetArrayLibrary.Array_AddUnique` _lamps (`self.Lamp5`))
  (`KismetArrayLibrary.Array_AddUnique` _lamps (`self.Lamp4`))
  (`KismetArrayLibrary.Array_AddUnique` _lamps (`self.Lamp3`))
  (`KismetArrayLibrary.Array_AddUnique` _lamps (`self.Lamp2`))
  (`KismetArrayLibrary.Array_AddUnique` _lamps (`self.Lamp1`))
  (`KismetArrayLibrary.Array_Resize` (`self.LampOn`) (`KismetArrayLibrary.Array_Length` (`self.Lamps`))))