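; Component that detects the interactable actor a controlled pawn is looking at.
; Each tick it runs a thin, short sphere trace forward from the camera on the Visibility channel and accepts hits implementing BPI_Interactable.
; A hit is flagged through SetSelectedMessage and stored as CurrentInteractable, which is deselected and cleared once the trace finds no interactable.
; CanInteract exposes whether a target exists and which actor it is.
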(event `self.ReceiveTick`
  (params (DeltaSeconds :type "Float (single-precision)"))
  (bind _camera (`self.Camera`))
  (bind _current_interactable (`self.Current Interactable`))
  (bind _returnvalue (`SceneComponent.K2_GetComponentLocation` _camera))
  (bind _outhit (`KismetSystemLibrary.SphereTraceSingle` _returnvalue (+ _returnvalue (* (`SceneComponent.GetForwardVector` _camera) 350.0)) 0.5 "TraceTypeQuery1"))
  (bind (_bblockinghit _binitialoverlap _time _distance _location _impactpoint _normal _impactnormal _physmat _hitactor) (`GameplayStatics.BreakHitResult` _outhit))
  (if (and (`KismetSystemLibrary.DoesImplementInterface` _hitactor "/Game/Blueprints/Interfaces/BPI_Interactable.BPI_Interactable_C") (`Pawn.IsPawnControlled` (cast `Pawn` (`self.GetOwner`) :!pure true)))
    (message `/Game/Blueprints/Interfaces/BPI_Interactable.SetSelected` _hitactor true)
    (set `self.Current Interactable` _hitactor)
    (else
      (`/Engine/EditorBlueprintResources/StandardMacros.IsValid` _current_interactable
        (:`Is Valid`
          (message `/Game/Blueprints/Interfaces/BPI_Interactable.SetSelected` _current_interactable false)
          (set `self.Current Interactable` null))))))

(fn `CanInteract`
  (returns (CanInteract :type Boolean) (CurrentInteractable :type "Actor Object Reference"))
  (bind _current_interactable (`self.Current Interactable`))
  (return (`KismetSystemLibrary.IsValid` _current_interactable) _current_interactable))