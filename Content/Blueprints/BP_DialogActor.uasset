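; BP_DialogActor is an interactable NPC that starts its current dialog through GM_FirstPersonGamemode, then sets it to "Silent".
; Tick shows a Cone whenever the dialog is not "Silent".
; GameStageUpdate uses per-stage maps to move NPCGraphic, swap the dialog and loop a Sit, Stand or Lie animation.
; Moves snap to a downward trace from the mapped actor and copy its rotation.
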(event EventGameStageUpdate
  (params (StageUpdated :type GameStages%20Enum :default "NewEnumerator3"))
  (bind _onstatemove (Variables|Default|GetOnStateMove))
  (bind _skeletalmesh (Variables|Default|GetSkeletalMesh))
  (bind _onstatedialogchange (Variables|Default|GetOnStateDialogChange))
  (bind _onstateanimchange (Variables|Default|GetOnStateAnimChange))
  (bind (_value _returnvalue) (Utilities|Map|Find _onstateanimchange StageUpdated))
  (bind (_value_2 _returnvalue_2) (Utilities|Map|Find _onstatemove StageUpdated))
  (bind (_value_3 _returnvalue_3) (Utilities|Map|Find _onstatedialogchange StageUpdated))
  (bind _returnvalue_4 (Transformation|GetActorLocation _value_2))
  (Utilities|FlowControl|Sequence
    (:then_0
      (if _returnvalue_2
        (bind _outhit (Collision|LineTraceByChannel _returnvalue_4 (- _returnvalue_4 "0.000000,0.000000,200.000000") "TraceTypeQuery1" false 0 "ForDuration"))
        (Transformation|SetWorldLocationAndRotation (Variables|Default|GetNPC_Graphic) (.location _outhit) (Transformation|GetActorRotation _value_2) false false)))
    (:then_1
      (if _returnvalue_3
        (Variables|Default|SetStartDialog _value_3)))
    (:then_2
      (if _returnvalue
        (if (== _value "Sit")
          (Components|Animation|PlayAnimation (Variables|Default|GetSkeletalMesh) "/Game/Blender/NPC/Sit.Sit" true)
          (Audio|Components|Audio|Play _skeletalmesh true :!label _label)
          (elif (== _value "Stand")
            (Components|Animation|PlayAnimation _skeletalmesh "/Game/Blender/NPC/Idle_.Idle_" true)
            (goto _label)
            (elif (== _value "Lie")
              (Components|Animation|PlayAnimation (Variables|Default|GetSkeletalMesh) "/Game/Blender/NPC/Lie.Lie" true)
              (goto _label)
              (else
                (Development|PrintString "NoAnim")))))))))

(event EventTick
  (params (DeltaSeconds :type Float%20%28single-precision%29))
  (bind _cone (Variables|Default|GetCone))
  (if (== (Variables|Default|GetStartDialog) "Silent")
    (Rendering|SetVisibility _cone false false)
    (else
      (Rendering|SetVisibility _cone true false))))

(event EventSetSelected
  (params (Selected :type Boolean)))

(event EventInteract
  (params (LastPossess :type Pawn%20Object%20Reference))
  (bind _asgm_first_person_gamemode (Utilities|Casting|CastToGM_FirstPersonGamemode (Game|GetGameMode)))
  (Default|StartDialog _asgm_first_person_gamemode (Variables|Default|GetStartDialog))
  (Variables|Default|SetStartDialog "Silent"))

(fn ConstructionScript)

(fn GetHeadPosition
  (return (Transformation|GetWorldLocation (Variables|Default|GetSphere))))

(fn Interactable
  (return true))