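; Interactable door that swings open and shut on alternate interactions with sound, and shows an overlay material while selected.
; A timeline lerps the root between its starting rotation and that of OpenPos, disabling door collision while it moves.
; The construction script yaws OpenPos by Rotation, with an optional debug mesh to preview the open position.
; Game stage updates enable or disable interaction at configured unlock and lock stages.
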(event `/Game/Blueprints/Interfaces/BPI_Interactable.SetSelected`
  (params (Selected :type Boolean))
  (bind _door (`self.Door`))
  (if Selected
    (`MeshComponent.SetOverlayMaterial` _door "/Game/Materials/Overlay/InteractMinimalist.InteractMinimalist")
    (else
      (`MeshComponent.SetOverlayMaterial` _door null))))

(event `/Game/Blueprints/Interfaces/BPI_Interactable.Interact`
  (params (LastPossess :type "Pawn Object Reference"))
  (bind _returnvalue (`self.K2_GetActorLocation`))
  (`/Engine/EditorBlueprintResources/StandardMacros.FlipFlop`
    (:`A`
      (`GameplayStatics.PlaySoundAtLocation` "/Game/Sounds/SFX/DoorOpen.DoorOpen" _returnvalue (struct) 1.0 1.0 0.0 null null null null)
      (bind (_direction _doorrotation) (`Timeline|OpeningDoor` :!label _label)
        (:`Update`
          (`SceneComponent.K2_SetWorldRotation` (`self.DefaultSceneRoot`) (`KismetMathLibrary.RLerp` (`self.ClosedWorldRot`) (`self.OpenWorldRot`) _doorrotation true) false false)
          (`PrimitiveComponent.SetCollisionEnabled` (`self.Door`) "NoCollision"))
        (:`Finished`
          (`PrimitiveComponent.SetCollisionEnabled` (`self.Door`) "QueryAndPhysics"))))
    (:`B`
      (`GameplayStatics.PlaySoundAtLocation` "/Game/Sounds/SFX/DoorClose.DoorClose" _returnvalue (struct) 1.0 1.0 0.0 null null null null)
      (goto _label :!via `Reverse`))))

(event `self.ReceiveBeginPlay`
  (set `self.ClosedWorldRot` (`SceneComponent.K2_GetComponentRotation` (`self.DefaultSceneRoot`)))
  (set `self.OpenWorldRot` (`SceneComponent.K2_GetComponentRotation` (`self.OpenPos`))))

(event `/Game/Blueprints/Interfaces/BPI_Interactable.SetCanInteract`
  (params (newInteractable :type Boolean))
  (set `self.CanInteract` newInteractable)
  (`KismetSystemLibrary.PrintString` "Hello"))

(event `/Game/Blueprints/Interfaces/BPI_GameStageListener.GameStageUpdate`
  (params (StageUpdated :type "/Game/Blueprints/DialogSystem/GameStages Enum" :default "NewEnumerator3"))
  (`|ExecutionSequence`
    (:`then_0`
      (if (`|EnumEquality` StageUpdated (`self.UnlockOnState`))
        (`/Game/Blueprints/Interfaces/BPI_Interactable.SetCanInteract` true)))
    (:`then_1`
      (if (`|EnumEquality` StageUpdated (`self.LockOnState`))
        (`/Game/Blueprints/Interfaces/BPI_Interactable.SetCanInteract` false)))))

(fn `Interactable`
  (returns (IsInteractable :type Boolean))
  (return (`self.CanInteract`)))

(fn `UserConstructionScript`
  (`SceneComponent.K2_SetRelativeRotation` (`self.OpenPos`) (`KismetMathLibrary.MakeRotator` 0.0 0.0 (`self.Rotation`)) false false)
  (`SceneComponent.SetVisibility` (`self.StaticMesh1`) (`self.DebugShowOpenPosition`) false))