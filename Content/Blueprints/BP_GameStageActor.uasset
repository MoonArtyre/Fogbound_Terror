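; BP_GameStageActor switches a set of ConnectedActors on or off as the game stage changes.
; GameStageUpdate compares the new stage to EnableOnGamestage and DisableOnGamestage, toggling tick, collision and visibility on each valid actor.
; Enabling sets hidden-in-game from the InVisible flag, so actors can become active while staying hidden.
; BeginPlay reuses the disable loop when DisableOnStart is set.
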(event `/Game/Blueprints/Interfaces/BPI_GameStageListener.GameStageUpdate`
  (params (StageUpdated :type "/Game/Blueprints/DialogSystem/GameStages Enum" :default "NewEnumerator3"))
  (`|ExecutionSequence`
    (:`then_0`
      (if (`|EnumEquality` (`self.EnableOnGamestage`) StageUpdated)
        (for _array_element (`self.ConnectedActors`)
          (`/Engine/EditorBlueprintResources/StandardMacros.IsValid` _array_element
            (:`Is Valid`
              (`self.SetActorTickEnabled` _array_element true)
              (`self.SetActorEnableCollision` _array_element true)
              (`self.SetActorHiddenInGame` _array_element (`self.InVisible`)))))))
    (:`then_1`
      (if (`|EnumEquality` StageUpdated (`self.DisableOnGamestage`))
        (for _array_element_2 (`self.ConnectedActors`) :!label _label
          (`/Engine/EditorBlueprintResources/StandardMacros.IsValid` _array_element_2
            (:`Is Valid`
              (`self.SetActorTickEnabled` _array_element_2 false)
              (`self.SetActorTickEnabled` _array_element_2 false)
              (`self.SetActorEnableCollision` _array_element_2 false)
              (`self.SetActorHiddenInGame` _array_element_2 true))))))))

(event `self.ReceiveBeginPlay`
  (if (`self.DisableOnStart`)
    (goto _label)))

(fn `UserConstructionScript`)