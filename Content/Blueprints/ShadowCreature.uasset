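; ShadowCreature is a scripted scare actor in which a shadow creature moves past when its trigger box is overlapped.
; On BeginPlay it records the creature's start and end locations and starts a looping play on the creature.
; The first overlap plays the Drone, calls FlashlightFlicker on BP_Player, and runs a Timeline that lerps the creature between those points before hiding it.
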(event `self.ReceiveBeginPlay`
  (set `self.StartTrans` (`SceneComponent.K2_GetComponentLocation` (`self.ShadowCreature`)))
  (set `self.EndTrans` (`SceneComponent.K2_GetComponentLocation` (`self.ShadowCreatureEnd`)))
  (`SkeletalMeshComponent.Play` (`self.ShadowCreature`) true))

(event `self.Box.OnComponentBeginOverlap`
  (params (OverlappedComponent :type "PrimitiveComponent Object Reference") (OtherActor :type "Actor Object Reference") (OtherComp :type "PrimitiveComponent Object Reference") (OtherBodyIndex :type Integer) (bFromSweep :type Boolean) (SweepResult :type "HitResult Structure (by ref)"))
  (bind _shadowcreature (`self.ShadowCreature`))
  (`/Engine/EditorBlueprintResources/StandardMacros.DoOnce` false
    (:`Completed`
      (`AudioComponent.Play` (`self.drone`) 0.3)
      (`|ExecutionSequence`
        (:`then_0`
          (bind (_direction _newtrack_0) (`Timeline|Timeline`)
            (:`Update`
              (`SceneComponent.K2_SetWorldLocation` _shadowcreature (`KismetMathLibrary.VLerp` (`self.StartTrans`) (`self.EndTrans`) _newtrack_0) false false))
            (:`Finished`
              (`SceneComponent.SetVisibility` _shadowcreature false false))))
        (:`then_1`
          (bind _returnvalue (`GameplayStatics.GetActorOfClass` "/Game/Blueprints/BP_Player.BP_Player_C"))
          (`/Game/Blueprints/BP_Player.Flashlight Flicker` _returnvalue))))))

(fn `UserConstructionScript`)