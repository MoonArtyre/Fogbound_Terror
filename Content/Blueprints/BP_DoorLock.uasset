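; BP_DoorLock is an interactable lock that unlocks another object when the player uses it.
; Selection toggles an overlay material on its cube, and a CanInteract flag, settable through SetCanInteract, is reported by Interactable.
; Interact sends SetCanInteract(true) to the Unlock reference, destroys the lock, then starts the "DoorBlackdade" dialog through GM_FirstPersonGamemode.
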(event `/Game/Blueprints/Interfaces/BPI_Interactable.SetSelected`
  (params (Selected :type Boolean))
  (if Selected
    (`MeshComponent.SetOverlayMaterial` (`self.Cube`) "/Game/Materials/Overlay/InteractMinimalist.InteractMinimalist")
    (else
      (`MeshComponent.SetOverlayMaterial` (`self.Cube`) null))))

(event `/Game/Blueprints/Interfaces/BPI_Interactable.Interact`
  (params (LastPossess :type "Pawn Object Reference"))
  (message `/Game/Blueprints/Interfaces/BPI_Interactable.SetCanInteract` (`self.Unlock`) true)
  (`self.K2_DestroyActor`)
  (bind _asgm_first_person_gamemode (cast `/Game/Blueprints/GM_FirstPersonGamemode` (`GameplayStatics.GetGameMode`)))
  (`/Game/Blueprints/GM_FirstPersonGamemode.StartDialog` _asgm_first_person_gamemode "DoorBlackdade"))

(event `/Game/Blueprints/Interfaces/BPI_Interactable.SetCanInteract`
  (params (newInteractable :type Boolean))
  (set `self.CanInteract` newInteractable))

(fn `Interactable`
  (returns (IsInteractable :type Boolean))
  (return (`self.CanInteract`)))

(fn `UserConstructionScript`)