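; Interactable lockpick minigame in which the player presses six pins in a shuffled order, hinted by each pin's height.
; Interact possesses the actor, swaps input mappings and shows the puzzle in front of a camera matched to the player's view.
; Correct picks raise pins, a mistake resets all, and both drive Lockpicking parameters.
; Solving or the cheat input returns control to the player and messages Unlock to allow interaction.
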(event `self.ReceiveBeginPlay`
  (bind _pinarray (`self.PinArray`))
  ;[1 1 1] Add Pins to array
  (`KismetArrayLibrary.Array_Add` _pinarray (`self.Pin`))
  (`KismetArrayLibrary.Array_Add` _pinarray (`self.Pin1`))
  (`KismetArrayLibrary.Array_Add` _pinarray (`self.Pin2`))
  (`KismetArrayLibrary.Array_Add` _pinarray (`self.Pin3`))
  (`KismetArrayLibrary.Array_Add` _pinarray (`self.Pin4`))
  (`KismetArrayLibrary.Array_Add` _pinarray (`self.Pin5`))
  (`self.Update Picker Pos`)
  (`SceneComponent.SetVisibility` (`self.LockpickPuzzle`) false true)
  (`self.RandomPuzzle`))

(event `EnhancedInput|/Game/Inputs/IA_Move`
  (params (ActionValue :type "Vector2D Structure") (ElapsedSeconds :type "Float (double-precision)") (TriggeredSeconds :type "Float (double-precision)") (InputAction :type "InputAction Object Reference" :default "/Game/Inputs/IA_Move.IA_Move"))
  (bind _returnvalue (+ (`self.CurrentPinSelection`) 1))
  (bind _returnvalue_2 (- (`self.CurrentPinSelection`) 1))
  ;[1 1 1] Move The Lockpicker
  (:`Started`
    (if (> ActionValue_X 0.0)
      (if (< _returnvalue (`KismetArrayLibrary.Array_Length` (`self.PinArray`)))
        (set `self.CurrentPinSelection` _returnvalue)
        (`self.Update Picker Pos` :!label _label))
      (elif (>= _returnvalue_2 0)
        (set `self.CurrentPinSelection` _returnvalue_2)
        (goto _label)))))

(event `EnhancedInput|/Game/Inputs/Keypad_Inputs/IA_Exit`
  (params (ActionValue :type Boolean) (ElapsedSeconds :type "Float (double-precision)") (TriggeredSeconds :type "Float (double-precision)") (InputAction :type "InputAction Object Reference" :default "/Game/Inputs/Keypad_Inputs/IA_Exit.IA_Exit"))
  ;[1 1 1] Exit
  (:`Started`
    (bind _asbp_player (cast `/Game/Blueprints/BP_Player` (`self.Last Possess`) :!label _label_2))
    (`/Game/Blueprints/BP_Player.Possess Player` _asbp_player)
    (`EnhancedInputSubsystemInterface.RemoveMappingContext` (pcsubsystem `EnhancedInputLocalPlayerSubsystem` (`GameplayStatics.GetPlayerController` 0)) "/Game/Inputs/IMC_Lockpick.IMC_Lockpick" (struct))
    (`SceneComponent.SetVisibility` (`self.LockpickPuzzle`) false true)))

(event `Exit`
  ;[1 1 1] Exit
  (goto _label_2))

(event `Update Picker Pos`
  ;[1 1 1] Update Picker Position
  (`SceneComponent.K2_SetRelativeLocation` (`self.Picker`) (+ (`SceneComponent.RelativeLocation` (`|GetArrayItem` (`self.PinArray`) (`self.CurrentPinSelection`))) (0.0 0.0 -20.0)) false false))

(event `/Game/Blueprints/Interfaces/BPI_Interactable.Interact`
  (params (LastPossess :type "Pawn Object Reference"))
  (bind _camera (`self.Camera`))
  (bind _lockpickpuzzle (`self.LockpickPuzzle`))
  (bind (_returnvalue_roll _returnvalue_pitch _returnvalue_yaw) (`KismetMathLibrary.BreakRotator` (`KismetMathLibrary.FindLookAtRotation` (`SceneComponent.K2_GetComponentLocation` _lockpickpuzzle) (`SceneComponent.K2_GetComponentLocation` (`self.Camera`)))))
  ;[1 1 1] Get Possessed
  (set `self.Last Possess` LastPossess)
  (bind _returnvalue (`GameplayStatics.GetActorOfClass` "/Game/Blueprints/BP_Player.BP_Player_C"))
  (`self.AddMappingFunction`)
  (`SceneComponent.K2_SetWorldTransform` (`self.Camera`) (`SceneComponent.K2_GetComponentToWorld` (`/Game/Blueprints/BP_Player.Camera` _returnvalue)) false false)
  (`/Game/Blueprints/BP_Macros.SmoothPosses` self 0.3
    (:`OUt`
      (message `/Game/Blueprints/Interfaces/BPI_Interactable.SetSelected` self false)
      (`SceneComponent.K2_SetWorldLocation` (`self.LockpickPuzzle`) (+ (`SceneComponent.K2_GetComponentLocation` _camera) (* (`SceneComponent.GetForwardVector` _camera) (`self.Distance From Cam`))) false false)
      (`SceneComponent.SetVisibility` (`self.LockpickPuzzle`) true true)
      (`SceneComponent.K2_SetWorldRotation` _lockpickpuzzle (`KismetMathLibrary.MakeRotator` _returnvalue_roll _returnvalue_pitch _returnvalue_yaw) false false))))

(event `EnhancedInput|/Game/Inputs/Keypad_Inputs/IA_Up`
  (params (ActionValue :type Boolean) (ElapsedSeconds :type "Float (double-precision)") (TriggeredSeconds :type "Float (double-precision)") (InputAction :type "InputAction Object Reference" :default "/Game/Inputs/Keypad_Inputs/IA_Up.IA_Up"))
  (bind _lockpicking (`self.Lockpicking`))
  (bind _lockpicking_2 (`self.Lockpicking`))
  ;[1 1 1] Pick Pn
  (:`Completed`
    (bind _returnvalue (`KismetArrayLibrary.Array_Add` (`self.Curent Guess`) (`self.CurrentPinSelection`)))
    (bind _output (`|GetArrayItem` (`self.Solution`) _returnvalue))
    (if (== (`|GetArrayItem` (`self.Curent Guess`) _returnvalue) _output)
      (bind _output_2 (`|GetArrayItem` (`self.PinArray`) _output))
      (`PrimitiveComponent.SetMaterial` _output_2 0 "/Game/Materials/M_Blockout_Opening.M_Blockout_Opening")
      (`SceneComponent.K2_AddRelativeLocation` _output_2 (0.0 0.0 5.0) false false)
      (`AudioParameterControllerInterface.SetFloatParameter` _lockpicking_2 "PinNumber" (`KismetMathLibrary.Conv_IntToDouble` (`KismetArrayLibrary.Array_Length` (`self.Curent Guess`))))
      (`AudioParameterControllerInterface.SetTriggerParameter` _lockpicking_2 "CorrectPin")
      (if (== (`KismetArrayLibrary.Array_Length` (`self.Solution`)) (`KismetArrayLibrary.Array_Length` (`self.Curent Guess`)))
        (set `self.Ineractable` false)
        (`self.Exit` :!label _label_3)
        (`self.Solved`)
        (`AudioParameterControllerInterface.SetTriggerParameter` (`self.Lockpicking`) "Solved"))
      (else
        (for _array_element (`self.PinArray`)
          (`PrimitiveComponent.SetMaterial` _array_element 0 "/Engine/BasicShapes/BasicShapeMaterial.BasicShapeMaterial")
          (bind (_relativelocation_x _relativelocation_y) (`KismetMathLibrary.BreakVector` (`SceneComponent.RelativeLocation` _array_element)))
          (`SceneComponent.K2_SetRelativeLocation` _array_element (`KismetMathLibrary.MakeVector` _relativelocation_x _relativelocation_y 10.0) false false))
        (`KismetArrayLibrary.Array_Clear` (`self.Curent Guess`))
        (`AudioParameterControllerInterface.SetTriggerParameter` _lockpicking "IncorrectPin")
        (`AudioParameterControllerInterface.SetFloatParameter` _lockpicking "PinNumber" 0.0)))))

(event `EnhancedInput|/Game/Inputs/IA_Cheat`
  (params (ActionValue :type Boolean) (ElapsedSeconds :type "Float (double-precision)") (TriggeredSeconds :type "Float (double-precision)") (InputAction :type "InputAction Object Reference" :default "/Game/Inputs/IA_Cheat.IA_Cheat"))
  ;[1 1 1] Pick Pn
  (:`Started`
    (goto _label_3)))

(event `/Game/Blueprints/Interfaces/BPI_Interactable.SetSelected`
  (params (Selected :type Boolean))
  ;[1 1 1] Select Highlight
  (if Selected
    (`MeshComponent.SetOverlayMaterial` (`self.LockpickObject`) "/Game/Materials/Overlay/InteractMinimalist.InteractMinimalist")
    (else
      (`MeshComponent.SetOverlayMaterial` (`self.LockpickObject`) null))))

(event `Solved`
  ;[1 1 1] OnSolved
  (`KismetSystemLibrary.PrintString` "Puzzle Solved")
  (message `/Game/Blueprints/Interfaces/BPI_Interactable.SetCanInteract` (`self.Unlock`) true)
  (`KismetSystemLibrary.Delay` 0.5))

(event `RandomPuzzle`
  (`KismetArrayLibrary.Array_Shuffle` (`self.Solution`))
  (for _index (range 6)
    (`SceneComponent.SetWorldScale3D` (`|GetArrayItem` (`self.PinArray`) (`|GetArrayItem` (`self.Solution`) _index)) (`KismetMathLibrary.MakeVector` 0.05 0.05 (+ (* (`KismetMathLibrary.Conv_IntToDouble` _index) 0.01) 0.1)))))

(fn `AddMappingFunction`
  (bind _returnvalue (pcsubsystem `EnhancedInputLocalPlayerSubsystem` (`GameplayStatics.GetPlayerController` 0)))
  (`/Engine/EditorBlueprintResources/StandardMacros.IsValid` _returnvalue
    (:`Is Valid`
      (`EnhancedInputSubsystemInterface.AddMappingContext` _returnvalue "/Game/Inputs/IMC_Lockpick.IMC_Lockpick" 0 (struct))
      (`EnhancedInputSubsystemInterface.RemoveMappingContext` _returnvalue "/Game/Inputs/IMC_Player.IMC_Player" (struct)))))

(fn `Interactable`
  (returns (IsInteractable :type Boolean))
  (return (`self.Ineractable`)))

(fn `UserConstructionScript`)