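; BP_Collectable is an interactable pickup that advances game dialog stages when collected, with its mesh and material applied in the construction script.
; Selection toggles a fresnel wave overlay material as a highlight.
; On interact, it adds and removes configured stages on GM_FirstPersonGamemode and starts an optional dialog.
; It then either destroys itself or disables further interaction and clears the highlight.
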(event `self.SetSelected`
  (params (Selected :type Boolean))
  (bind _collectablemesh (`self.CollectableMesh`))
  (if Selected
    (`MeshComponent.SetOverlayMaterial` _collectablemesh "/Game/Materials/Overlay/M_FresnelWave.M_FresnelWave")
    (else
      (`MeshComponent.SetOverlayMaterial` _collectablemesh null))))

(event `self.Interact`
  (params (LastPossess :type "Pawn Object Reference"))
  (bind _playdialogoncollect (`self.PlayDialogOnCollect`))
  (bind _asgm_first_person_gamemode (cast `/Game/Blueprints/GM_FirstPersonGamemode` (`GameplayStatics.GetGameMode`)))
  (for _array_element (`self.DialogStagesToAdd`)
    (`/Game/Blueprints/GM_FirstPersonGamemode.Add GameStage` _asgm_first_person_gamemode _array_element))
  (for _array_element_2 (`self.DialogStagesToRemove`)
    (`/Game/Blueprints/GM_FirstPersonGamemode.Remove GameStage` _asgm_first_person_gamemode _array_element_2))
  (bind _asgm_first_person_gamemode_2 (cast `/Game/Blueprints/GM_FirstPersonGamemode` (`GameplayStatics.GetGameMode`))
    (:`then`
      (if (not (== _playdialogoncollect "None"))
        (`/Game/Blueprints/GM_FirstPersonGamemode.StartDialog` _asgm_first_person_gamemode_2 _playdialogoncollect)))
    (:`CastFailed`
      _))
  (if (`self.DestroyObjectOnCollect`)
    (`self.K2_DestroyActor`)
    (else
      (`self.SetCanInteract` false)
      (`self.SetSelected` false))))

(event `self.SetCanInteract`
  (params (newInteractable :type Boolean))
  (set `self.isInteractable` newInteractable))

(fn `Interactable`
  (returns (IsInteractable :type Boolean))
  (return (`self.isInteractable`)))

(fn `UserConstructionScript`
  (bind _collectablemesh (`self.CollectableMesh`))
  (`StaticMeshComponent.SetStaticMesh` _collectablemesh (`self.Mesh`))
  (`PrimitiveComponent.SetMaterial` _collectablemesh 0 (`self.Material`)))